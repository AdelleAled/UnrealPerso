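; BP_Pile is a procedural prop that builds a vertical pile of static meshes picked at random from ObjectList.
; The Construction Script adds ObjectCount components, stacking each by bounding-box height times a tuning multiplier, with random Y offset and yaw.
; Random negative scale on each axis mirrors pieces for variety, and unseeded randomness reshuffles the pile on each reconstruction.
; The event graph is empty, and the TopObject placement logic is disconnected.
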(event EventBeginPlay)

(event Collision|EventActorBeginOverlap
  (params (OtherActor :type Actor%20Object%20Reference)))

(event EventTick
  (params (DeltaSeconds :type Float%20%28single-precision%29)))

(fn ConstructionScript
  (bind _returnvalue (Math|Random|RandomBool))
  (bind _returnvalue_2 (Math|Conversions|ToFloat(Boolean) _returnvalue))
  (bind _returnvalue_3 (Math|Float|Lerp 1.0 -1.0 _returnvalue_2))
  (for _index (range 0 (Variables|Default|GetObjectCount))
    (bind _output_get (LocalVariables|SetCurrentStaticMeshToAdd (.OutItem (Utilities|Array|Random (Variables|Default|GetObjectList)))))
    (bind _output_get_2 (LocalVariables|SetCurrentObjectThickness (* (Utilities|Operators|Subtract (.z (.max (StaticMesh|GetBoundingBox _output_get))) (.z (.min (StaticMesh|GetBoundingBox _output_get)))) (Variables|Default|GetBoundingBoxVariable))))
    (bind _returnvalue_4 (AddComponent|AddStaticMeshComponent false (Math|Transform|MakeTransform (Math|Vector|MakeVector 0.0 (Math|Random|RandomFloatinRange (Variables|Default|GetMin%20Position) (Variables|Default|GetMax%20Position)) (+ (/ _output_get_2 2.0) (LocalVariables|GetCurrentTotalObjectHeigh))) (Math|Rotator|MakeRotator 0.0 0.0 (Math|Random|RandomFloatinRange (Variables|Default|GetMin%20Rotation) (Variables|Default|GetMax%20Rotation))) (Math|Vector|MakeVector _returnvalue_3 _returnvalue_3 _returnvalue_3))))
    (AddComponent|AddStaticMeshComponent false)
    (Components|StaticMesh|SetStaticMesh _returnvalue_4 (LocalVariables|GetCurrentStaticMeshToAdd))
    (LocalVariables|SetCurrentTotalObjectHeigh (+ (LocalVariables|GetCurrentObjectThickness) (LocalVariables|GetCurrentTotalObjectHeigh)))))